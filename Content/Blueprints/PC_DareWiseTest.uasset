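; Player controller that owns the WBP_HUD widget and flags whether its possessed pawn is player 1.
; It creates the HUD on BeginPlay, then forwards custom events for cube type, cube data visibility, cube count, warnings and energy to that widget.
; On possession it sets IsPlayer1 on BP_Player_BaseClass pawns by checking whether the controller's own display name contains "1".
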(event Custom|SetupHUD
  ;[1 1 1] Create HUD
  (bind _returnvalue (UserInterface|CreateWidget "/Game/UI/WBP_Hud.WBP_HUD_C" self))
  (bind _output_get (Variables|Default|SetHUD_Reference _returnvalue))
  (UserInterface|Viewport|AddtoViewport _output_get 0))

(event EventBeginPlay
  (CallFunction|SetupHUD))

(event EventPossess
  (params (PossessedPawn :type Pawn%20Object%20Reference))
  ;[1 1 1] Setting player 1
  (bind _asbp_player_base_class (Utilities|Casting|CastToBP_Player_BaseClass PossessedPawn))
  (Variables|/Game/Blueprints/BP_Player_BaseClass.BP_Player_BaseClass_C|SetIsPlayer1? _asbp_player_base_class (Utilities|String|Contains (Utilities|GetDisplayName self) "1")))

(event EventUpdateCubeTypeDisplay
  (params (CubeIndex :type Integer))
  ;[1 1 1] HUD Function Calls
  (Default|SetCubeData (Variables|Default|GetHUD_Reference) CubeIndex))

(event EventShowCubeData
  ;[1 1 1] HUD Function Calls
  (Default|ShowCubeData (Variables|Default|GetHUD_Reference)))

(event EventHideCubeData
  ;[1 1 1] HUD Function Calls
  (Default|HideCubeData (Variables|Default|GetHUD_Reference)))

(event EventUpdateNumberOfCubesinLevel
  (params (NumberOfCubes :type Integer))
  ;[1 1 1] HUD Function Calls
  (Default|SetNumberOfCubesPlaced (Variables|Default|GetHUD_Reference) NumberOfCubes))

(event EventWarningMessage
  (params (MessageIndex :type Integer))
  ;[1 1 1] HUD Function Calls
  (Default|DisplayWarningMessage (Variables|Default|GetHUD_Reference) MessageIndex))

(event EventUpdateEnergyBarHUD
  (params (Energy :type Float%20%28single-precision%29))
  ;[1 1 1] HUD Function Calls
  (Default|SetEnergyBarPercent (Variables|Default|GetHUD_Reference) Energy))

(fn ConstructionScript)