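; Base cube Blueprint that tints itself by network authority and changes its solidity based on energy cost.
; The construction script creates a dynamic material instance on the cube mesh.
; On BeginPlay, SetValues applies the first-player tint with authority or the second-player tint without it.
; Cubes at or above the energy cost threshold become mostly transparent and ignore Pawn collision.
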(event Custom|SetValues
  (if (Variables|Default|GetAuthority?)
    (Rendering|Material|SetVectorParameterValue (Variables|Default|GetMaterialInstance) "Color" (Variables|Default|Get1stPlayerCubeTint) :!class /Script/Engine.MaterialInstanceDynamic)
    (else
      (Rendering|Material|SetVectorParameterValue (Variables|Default|GetMaterialInstance) "Color" (Variables|Default|Get2ndPlayerCubeTint) :!class /Script/Engine.MaterialInstanceDynamic)))
  (if (>= (Variables|Default|GetEnergyCost) 5e+01)
    (Rendering|Material|SetScalarParameterValue (Variables|Default|GetMaterialInstance) "Opacity" 0.3 :!class /Script/Engine.MaterialInstanceDynamic)
    (Collision|SetCollisionResponsetoChannel (Variables|Default|GetCube) "ECC_Pawn" "ECR_Ignore")))

(event EventBeginPlay
  (CallFunction|SetValues))

(event Collision|EventActorBeginOverlap
  (params (OtherActor :type Actor%20Object%20Reference)))

(event EventTick
  (params (DeltaSeconds :type Float%20%28single-precision%29)))

(fn ConstructionScript
  (bind _returnvalue (Rendering|Material|CreateDynamicMaterialInstance (Variables|Default|GetCube) 0 0 "None" :!class /Script/Engine.PrimitiveComponent))
  (Variables|Default|SetMaterialInstance _returnvalue))